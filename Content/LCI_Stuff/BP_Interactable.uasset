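; BP_Interactable is an interactable actor that shows a prompt and arms a dialogue UI while its box is overlapped.
; BeginPlay caches the first-person character; any overlap, unfiltered by actor, enables its interaction, sets WBP_DialogueOptions as its UI to open and shows a newly created prompt widget with InteractionText.
; Ending overlap disables interaction, calls the empty EndInteractionPrompt event, removes the player's UI and hides the prompt.
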(event `self.ReceiveBeginPlay`
  (bind _returnvalue (`GameplayStatics.GetActorOfClass` "/Game/FirstPerson/Blueprints/BP_FirstPersonCharacter.BP_FirstPersonCharacter_C"))
  (set `self.PlayerRef` _returnvalue))

(event `self.Box.OnComponentBeginOverlap`
  (params (OverlappedComponent :type "PrimitiveComponent Object Reference") (OtherActor :type "Actor Object Reference") (OtherComp :type "PrimitiveComponent Object Reference") (OtherBodyIndex :type Integer) (bFromSweep :type Boolean) (SweepResult :type "HitResult Structure (by ref)"))
  (set `/Game/FirstPerson/Blueprints/BP_FirstPersonCharacter.CanInteract` true (`self.PlayerRef`))
  (bind _returnvalue (`|CreateWidget` "/Game/LCI_Stuff/WBP_InteractionPrompt.WBP_InteractionPrompt_C"))
  (bind _output_get (set `self.InteractWidget` _returnvalue))
  (`WidgetComponent.SetWidget` (`self.Widget`) _output_get)
  (set `/Game/LCI_Stuff/WBP_InteractionPrompt.Text` (`self.InteractionText`) (`self.InteractWidget`))
  (set `self.Inside` true)
  (set `/Game/FirstPerson/Blueprints/BP_FirstPersonCharacter.UiToOpen` "/Game/LCI_Stuff/Dialogue/WBP_DialogueOptions.WBP_DialogueOptions_C" (`self.PlayerRef`))
  (`SceneComponent.SetHiddenInGame` (`self.Widget`) false false))

(event `EndInteractionPrompt`)

(event `self.Box.OnComponentEndOverlap`
  (params (OverlappedComponent :type "PrimitiveComponent Object Reference") (OtherActor :type "Actor Object Reference") (OtherComp :type "PrimitiveComponent Object Reference") (OtherBodyIndex :type Integer))
  (bind _playerref (`self.PlayerRef`))
  (set `/Game/FirstPerson/Blueprints/BP_FirstPersonCharacter.CanInteract` false _playerref)
  (set `self.Inside` false)
  (`self.EndInteractionPrompt`)
  (`/Game/FirstPerson/Blueprints/BP_FirstPersonCharacter.RemoveUi` _playerref)
  (`SceneComponent.SetHiddenInGame` (`self.Widget`) true false))

(fn `UserConstructionScript`)