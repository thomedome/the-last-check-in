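; Slot machine puzzle interactable that needs the player's collected lever and pays out a guaranteed, one-time reward.
; The first interaction attaches the lever with timelines that fade and slide it in; the next pulls it.
; Looping timers spin three reels at different speeds, then staggered delays stop each at zero rotation.
; A BP_Reward spawns after the second reel stops, gets an impulse, then has physics disabled.
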(event `self.ReceiveBeginPlay`
  ;[1 0.8849 0.1165] Gets A Reference To Player And The Levers Start Location
  (bind _returnvalue (`GameplayStatics.GetActorOfClass` "/Game/Eben_Work/BP_FirstPersonCharacterEben.BP_FirstPersonCharacterEben_C"))
  (set `self.Player Ref` _returnvalue)
  (set `self.Lever Start Location` (`SceneComponent.RelativeLocation` (`self.Lever Ancor`))))

(event `/Game/tomWork/Interfaces/IF_Interactable.ProcInteract`
  (params (hitComponent :type "PrimitiveComponent Object Reference"))
  (bind _lever (`self.Lever`))
  ;[0.5462 1 0] Interaction Event And Conditions
  (if (`/Game/Eben_Work/BP_FirstPersonCharacterEben.Lever Collected?` (`self.Player Ref`))
    (if (`self.Lever Attached?`)
      ;[0.1514 1 0.3143] Lever Pulling Timeline And Rotation Lerp
      (bind (_direction _alpha) (`Timeline|Lever Timeline`)
        (:`Update`
          (`SceneComponent.K2_SetRelativeRotation` (`self.Lever Ancor`) (`KismetMathLibrary.RLerp` (struct :`Pitch` 70.0 :`Yaw` 90.0 :`Roll` 90.0) (struct :`Pitch` 20.0 :`Yaw` 90.0 :`Roll` 90.0) _alpha) false false)
          (`KismetSystemLibrary.Delay` 0.65)
          ;[1 0.3384 0.9621] Blueprint For Reel Movement And Stopping The Reels After 4 Seconds
          (`/Engine/EditorBlueprintResources/StandardMacros.DoOnce` false
            (:`Completed`
              (`self.Stop Reels`)
              (bind _returnvalue (`KismetSystemLibrary.K2_SetTimerDelegate` (delegate `Rotate Reel 1`) 0.001 true))
              (set `self.Stop Reel 1` _returnvalue)
              (bind _returnvalue_2 (`KismetSystemLibrary.K2_SetTimerDelegate` (delegate `Rotate Reel 2`) 0.00125 true))
              (set `self.Stop Reel 2` _returnvalue_2)
              (bind _returnvalue_3 (`KismetSystemLibrary.K2_SetTimerDelegate` (delegate `Rotate Reel 3`) 0.0015 true))
              (set `self.Stop Reel 3` _returnvalue_3)))))
      (else
        ;[0.9913 0.6924 1] Logic Before Preforming Lever Attatchment Code
        (`/Engine/EditorBlueprintResources/StandardMacros.DoOnce` false
          (:`Completed`
            (`SceneComponent.SetHiddenInGame` (`self.Lever`) false false)
            (`|ExecutionSequence`
              (:`then_0`
                ;[1 0.8712 0.1183] Moves The Lever When It Is Attached, Lerps Its Transparency And Sets The Boolean To True
                (bind (_direction_2 _transparency_alpha) (`Timeline|Lever Attach Timeline` :!via `PlayFromStart`)
                  (:`Update`
                    (`MeshComponent.SetScalarParameterValueOnMaterials` _lever "Transparency" _transparency_alpha))
                  (:`Finished`
                    (`PrimitiveComponent.SetMaterial` _lever 0 "/Game/ollieWork/Slot_Machine/M_White.M_White")
                    (set `self.Lever Attached?` true))))
              (:`then_1`
                (bind (_direction_3 _transparency_alpha_2) (`Timeline|Lever Movement Timline` :!via `PlayFromStart`)
                  (:`Update`
                    (`SceneComponent.K2_SetRelativeLocation` (`self.Lever Ancor`) (`KismetMathLibrary.VLerp` (`self.Lever Start Location`) (- (`self.Lever Start Location`) (70.0 0.0 0.0)) _transparency_alpha_2) false false)))))))))))

(event `Rotate Reel 2`
  (bind (_relativerotation_roll _relativerotation_pitch _relativerotation_yaw) (`KismetMathLibrary.BreakRotator` (`SceneComponent.RelativeRotation` (`self.Reel 2`))))
  ;[1 0.3384 0.9621] Blueprint For Reel Movement And Stopping The Reels After 4 Seconds
  (`SceneComponent.K2_SetRelativeRotation` (`self.Reel 2`) (`KismetMathLibrary.MakeRotator` _relativerotation_roll _relativerotation_pitch (+ _relativerotation_yaw 1.0)) false false))

(event `Rotate Reel 3`
  (bind (_relativerotation_roll _relativerotation_pitch _relativerotation_yaw) (`KismetMathLibrary.BreakRotator` (`SceneComponent.RelativeRotation` (`self.Reel 3`))))
  ;[1 0.3384 0.9621] Blueprint For Reel Movement And Stopping The Reels After 4 Seconds
  (`SceneComponent.K2_SetRelativeRotation` (`self.Reel 3`) (`KismetMathLibrary.MakeRotator` _relativerotation_roll _relativerotation_pitch (+ _relativerotation_yaw 1.0)) false false))

(event `Rotate Reel 1`
  (bind (_relativerotation_roll _relativerotation_pitch _relativerotation_yaw) (`KismetMathLibrary.BreakRotator` (`SceneComponent.RelativeRotation` (`self.Reel 1`))))
  ;[1 0.3384 0.9621] Blueprint For Reel Movement And Stopping The Reels After 4 Seconds
  (`SceneComponent.K2_SetRelativeRotation` (`self.Reel 1`) (`KismetMathLibrary.MakeRotator` _relativerotation_roll _relativerotation_pitch (+ _relativerotation_yaw 1.0)) false false))

(event `Stop Reels`
  ;[1 0.008681 0] Stops The Reels Rotation And Starts The Code For Spawning The Reward
  (`KismetSystemLibrary.Delay` 4.0)
  (`|ExecutionSequence`
    (:`then_0`
      (`KismetSystemLibrary.Delay` 0.5)
      (`KismetSystemLibrary.K2_ClearAndInvalidateTimerHandle` (`self.Stop Reel 1`))
      (`SceneComponent.K2_SetRelativeRotation` (`self.Reel 1`) (`KismetMathLibrary.MakeRotator` 0.0) false false))
    (:`then_1`
      (`KismetSystemLibrary.Delay` 1.0)
      (`KismetSystemLibrary.K2_ClearAndInvalidateTimerHandle` (`self.Stop Reel 2`))
      (`SceneComponent.K2_SetRelativeRotation` (`self.Reel 2`) (`KismetMathLibrary.MakeRotator` 0.0) false false)
      (`KismetSystemLibrary.Delay` 0.4)
      ;[1 0.8446 0] Spawns The Reward And Stops Its Movment After A Delay.
      (bind _returnvalue (`|SpawnActorFromClass` "/Game/ollieWork/Slot_Machine/BP_Reward.BP_Reward_C" (`KismetMathLibrary.MakeTransform` (`SceneComponent.K2_GetComponentLocation` (`self.Reward`))) "Undefined" "MultiplyWithRoot" null null))
      (bind _cylinder (`/Game/ollieWork/Slot_Machine/BP_Reward.Cylinder` _returnvalue))
      (`PrimitiveComponent.AddImpulse` _cylinder (0.0 0.0 40.0) "None" false)
      (`KismetSystemLibrary.Delay` 1.25)
      (`PrimitiveComponent.SetSimulatePhysics` _cylinder false))
    (:`then_2`
      (`KismetSystemLibrary.Delay` 1.5)
      (`KismetSystemLibrary.K2_ClearAndInvalidateTimerHandle` (`self.Stop Reel 3`))
      (`SceneComponent.K2_SetRelativeRotation` (`self.Reel 3`) (`KismetMathLibrary.MakeRotator` 0.0) false false))))

(fn `UserConstructionScript`
  (bind _returnvalue (`PrimitiveComponent.CreateDynamicMaterialInstance` (`self.Lever`) 0 "/Game/ollieWork/Slot_Machine/M_Opacity.M_Opacity" "None"))
  (set `self.Material` _returnvalue))