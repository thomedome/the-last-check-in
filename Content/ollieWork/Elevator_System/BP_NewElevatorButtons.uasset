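; Elevator button panel that sends BP_Elevator to the floor stored in the pressed button's component tag.
; Floor calls require the secret button: interacting with a button attaches it via a timeline once the player has collected it, then stops the sparks.
; Later presses, blocked during lift cooldown or for the current floor, animate the button, reset the previous one and move the glow using dynamic materials.
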(event `self.ReceiveBeginPlay`
  ;[0 1 0.3505] Places Buttons In An Array For Location Reseting And Gets Other Actors For Refrence
  (set `self.Button Array` (`|MakeArray` (`self.Button_1`) (`self.Button_2`)))
  (bind _returnvalue (`GameplayStatics.GetActorOfClass` "/Game/tomWork/TemplateContent/FirstPerson/Blueprints/BP_FirstPersonCharacter.BP_FirstPersonCharacter_C"))
  (set `self.playerRef` _returnvalue)
  (bind _returnvalue_2 (`GameplayStatics.GetActorOfClass` "/Game/ollieWork/Elevator_System/BP_Elevator.BP_Elevator_C"))
  (set `self.elevatorRef` _returnvalue_2)
  (set `self.Button Start Location` (`SceneComponent.RelativeLocation` (`self.Button_2`))))

(event `Reset Button Locations`
  ;[1 0 0.08926] Resets Button Positions When Another Button Is Pressed
  (`SceneComponent.K2_SetRelativeLocation` (`self.Target Button`) (`self.Button Unpressed Location`) false false)
  ;[1 0.2882 0] Handles Button Glow Values
  (`MaterialInstanceDynamic.SetScalarParameterValue` (`self.Light Material 1`) "Light Value" 0.0)
  (`MaterialInstanceDynamic.SetScalarParameterValue` (`self.Light Material 2`) "Light Value" 0.0)
  (`MaterialInstanceDynamic.SetScalarParameterValue` (`self.Lit Button Material`) "Light Value" 1.0))

(event `/Game/tomWork/Interfaces/IF_Interactable.ProcInteract`
  (params (hitComponent :type "PrimitiveComponent Object Reference"))
  ;[0 0.3307 1] Validate Player Request
  (set `self.Hit Component` hitComponent)
  (if (`ActorComponent.ComponentHasTag` hitComponent "Button")
    (set `self.calledFloor` (`KismetStringLibrary.Conv_StringToInt` (`KismetStringLibrary.Conv_NameToString` (`|GetArrayItem` (`ActorComponent.ComponentTags` (`self.Hit Component`)) 1))))
    (if (== (`self.calledFloor`) (`/Game/ollieWork/Elevator_System/BP_Elevator.currentFloor` (`self.elevatorRef`)))
      _
      (elif (`self.Secret Button Attached?`)
        (if (not (`/Game/ollieWork/Elevator_System/BP_Elevator.Lift Cooldown` (`self.elevatorRef`)))
          (`/Engine/EditorBlueprintResources/StandardMacros.IsValid` (`self.Target Button`)
            (:`Is Valid`
              (`self.Reset Button Locations`))
            (:`Is Not Valid`
              _))
          (bind _output_get (set `self.Target Button` (`self.Hit Component`)))
          (set `self.Button Unpressed Location` (`SceneComponent.RelativeLocation` (`self.Target Button`)))
          (`|ExecutionSequence`
            (:`then_0`
              (bind _asmaterial_instance_dynamic (cast `MaterialInstanceDynamic` (`PrimitiveComponent.GetMaterial` _output_get 0)))
              ;[0.7383 0 1] Change Pressed Button Material
              (`MaterialInstanceDynamic.SetScalarParameterValue` _asmaterial_instance_dynamic "Light Value" 1.0)
              (set `self.Lit Button Material` _asmaterial_instance_dynamic)
              ;[1 0.06055 0] Call Go To Floor Event And Reset Button Glow / Locations
              (`/Game/ollieWork/Elevator_System/BP_Elevator.goToFloor` (`self.elevatorRef`) (`self.calledFloor`))
              (`self.Reset Button Locations`))
            (:`then_1`
              (set `self.Button Unpressed Location` (`SceneComponent.RelativeLocation` (`self.Target Button`)))
              ;[1 0.9032 0.1896] Button Movement Timeline
              (bind (_direction _button_alpha) (`Timeline|Button Click`)
                (:`Update`
                  (`SceneComponent.K2_SetRelativeLocation` (`self.Target Button`) (`KismetMathLibrary.VLerp` (`self.Button Unpressed Location`) (- (`self.Button Unpressed Location`) (0.0 4.0 0.0)) _button_alpha) false false))))))
        (elif (`/Game/tomWork/TemplateContent/FirstPerson/Blueprints/BP_FirstPersonCharacter.Button Collected?` (`self.playerRef`))
          (`self.Attach Button`))))))

(event `Attach Button`
  (bind _button_2 (`self.Button_2`))
  (`SceneComponent.SetHiddenInGame` (`self.Button_2`) false false)
  (`SceneComponent.SetHiddenInGame` (`self.2`) false false)
  (bind (_direction _alpha) (`Timeline|Button Timeline`)
    (:`Update`
      (`SceneComponent.K2_SetRelativeLocation` _button_2 (`KismetMathLibrary.VLerp` (`self.Button Start Location`) (- (`self.Button Start Location`) (0.0 23.0 0.0)) _alpha) false false))
    (:`Finished`
      (set `self.Secret Button Attached?` true)
      (set `self.Button Unpressed Location` (`SceneComponent.RelativeLocation` _button_2))
      (`ActorComponent.Deactivate` (`self.NS_Sparks`)))))

(fn `UserConstructionScript`
  (bind _returnvalue (`PrimitiveComponent.CreateDynamicMaterialInstance` (`self.Button_1`) 0 "/Game/ollieWork/Materials/M_ButtonLight.M_ButtonLight" "None"))
  (set `self.Light Material 1` _returnvalue)
  (bind _returnvalue_2 (`PrimitiveComponent.CreateDynamicMaterialInstance` (`self.Button_2`) 0 "/Game/ollieWork/Materials/M_ButtonLight.M_ButtonLight" "None"))
  (set `self.Light Material 2` _returnvalue_2))