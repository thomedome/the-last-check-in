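; Four-button elevator panel that lights and presses the selected button and triggers the matching floor event.
; An interaction interface event, ignored during BP_Elevator's LiftCooldown, maps the interact state to a button and calls that floor's event on BP_FirstPersonCharacter.
; Each press resets all buttons, keeps the selected one lit through per-button dynamic materials, and plays a timeline that pushes it in.
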(event `Reset Button Locations`
  ;[1 0 0.08926] Resets Button Positions When Another Button Is Pressed
  (for _array_element (`self.Button Array`)
    (`SceneComponent.K2_SetRelativeLocation` _array_element (0.0 0.0 0.0) false false)
    ;[1 0.2882 0] Handles Button Glow Values
    (`MaterialInstanceDynamic.SetScalarParameterValue` (`self.Light Material 1`) "Light Value" 0.0)
    (`MaterialInstanceDynamic.SetScalarParameterValue` (`self.Light Material 2`) "Light Value" 0.0)
    (`MaterialInstanceDynamic.SetScalarParameterValue` (`self.Light Material 3`) "Light Value" 0.0)
    (`MaterialInstanceDynamic.SetScalarParameterValue` (`self.Light Material 4`) "Light Value" 0.0)
    (`MaterialInstanceDynamic.SetScalarParameterValue` (`self.Lit Button`) "Light Value" 1.0)))

(event `self.ReceiveBeginPlay`
  ;[0 1 0.3505] Places Buttons In An Array For Location Reseting And Gets Other Actors For Refrence
  (set `self.Button Array` (`|MakeArray` (`self.Button_1`) (`self.Button_2`) (`self.Button_3`) (`self.Button_4`)))
  (bind _returnvalue (`GameplayStatics.GetActorOfClass` "/Game/ollieWork/Elevator_System/BP_Elevator.BP_Elevator_C"))
  (bind _returnvalue_2 (`GameplayStatics.GetActorOfClass` "/Game/tomWork/TemplateContent/FirstPerson/Blueprints/BP_FirstPersonCharacter.BP_FirstPersonCharacter_C")))

(event `/Game/ollieWork/Elevator_System/BPI_InteractionObjects.BPI_InteractObject`
  (params (InteractState :type String))
  (bind _light_material_1 (`self.Light Material 1`))
  (bind _light_material_2 (`self.Light Material 2`))
  (bind _light_material_3 (`self.Light Material 3`))
  (bind _light_material_4 (`self.Light Material 4`))
  ;[1 0 0.009094] Checks What Button Has Been Hit By The Ray-Trace Using The Interacton Function And Places It Into A Variable
  (if (not (`/Game/ollieWork/Elevator_System/BP_Elevator.Lift Cooldown` (stale `self.ReceiveBeginPlay` _returnvalue)))
    (bind _output_get (set `self.Interact State` InteractState))
    (`|ExecutionSequence`
      (:`then_0`
        (switch `string` _output_get
          (:`Button_1`
            (set `self.Target Button` (`self.Button_1`))
            ;[0.7383 0 1] Lights Up Hit Button
            (`MaterialInstanceDynamic.SetScalarParameterValue` _light_material_1 "Light Value" 1.0)
            (set `self.Lit Button` _light_material_1)
            ;[0 0.3389 1] Fires Elevator Custom Events And Resets Button Glow And Locations
            (`/Game/tomWork/TemplateContent/FirstPerson/Blueprints/BP_FirstPersonCharacter.First Floor` (stale `self.ReceiveBeginPlay` _returnvalue_2)))
          (:`Button_2`
            (set `self.Target Button` (`self.Button_2`))
            (`MaterialInstanceDynamic.SetScalarParameterValue` _light_material_2 "Light Value" 1.0)
            (set `self.Lit Button` _light_material_2)
            (`/Game/tomWork/TemplateContent/FirstPerson/Blueprints/BP_FirstPersonCharacter.Second Floor` (stale `self.ReceiveBeginPlay` _returnvalue_2)))
          (:`Button_3`
            (set `self.Target Button` (`self.Button_3`))
            (`MaterialInstanceDynamic.SetScalarParameterValue` _light_material_3 "Light Value" 1.0)
            (set `self.Lit Button` _light_material_3)
            (`/Game/tomWork/TemplateContent/FirstPerson/Blueprints/BP_FirstPersonCharacter.Third Floor` (stale `self.ReceiveBeginPlay` _returnvalue_2)))
          (:`Button_4`
            (set `self.Target Button` (`self.Button_4`))
            (`MaterialInstanceDynamic.SetScalarParameterValue` _light_material_4 "Light Value" 1.0)
            (set `self.Lit Button` _light_material_4)
            (`/Game/tomWork/TemplateContent/FirstPerson/Blueprints/BP_FirstPersonCharacter.Fourth Floor` (stale `self.ReceiveBeginPlay` _returnvalue_2))))
        (`self.Reset Button Locations`))
      (:`then_1`
        ;[1 0.9032 0.1896] Button Movement Timeline
        (bind (_direction _button_alpha) (`Timeline|Button Click` :!via `PlayFromStart`)
          (:`Update`
            (`SceneComponent.K2_SetRelativeLocation` (`self.Target Button`) (`KismetMathLibrary.VLerp` (0.0 0.0 0.0) (0.0 -4.0 0.0) _button_alpha) false false)))))))

(fn `UserConstructionScript`
  (bind _returnvalue (`PrimitiveComponent.CreateDynamicMaterialInstance` (`self.Button_1`) 0 "/Game/ollieWork/Materials/M_ButtonLight.M_ButtonLight" "None"))
  (set `self.Light Material 1` _returnvalue)
  (bind _returnvalue_2 (`PrimitiveComponent.CreateDynamicMaterialInstance` (`self.Button_2`) 0 "/Game/ollieWork/Materials/M_ButtonLight.M_ButtonLight" "None"))
  (set `self.Light Material 2` _returnvalue_2)
  (bind _returnvalue_3 (`PrimitiveComponent.CreateDynamicMaterialInstance` (`self.Button_3`) 0 "/Game/ollieWork/Materials/M_ButtonLight.M_ButtonLight" "None"))
  (set `self.Light Material 3` _returnvalue_3)
  (bind _returnvalue_4 (`PrimitiveComponent.CreateDynamicMaterialInstance` (`self.Button_4`) 0 "/Game/ollieWork/Materials/M_ButtonLight.M_ButtonLight" "None"))
  (set `self.Light Material 4` _returnvalue_4))