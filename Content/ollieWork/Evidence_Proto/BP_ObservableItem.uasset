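; Inspectable item, optionally flagged as evidence, that the player can zoom in on and observe.
; Sphere overlap places a shared BP_Camera at the item, sizing arm length and raise height from mesh bounds.
; Interacting freezes the player, blends to that camera, then timeline-raises the mesh before enabling observation; lowering restores rotation.
; A dynamic white-outline overlay material provides the highlight, faded via timeline on overlap end.
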(event `/Game/tomWork/Interfaces/IF_Interactable.ProcInteract`
  (params (hitComponent :type "PrimitiveComponent Object Reference"))
  (bind _returnvalue (`GameplayStatics.GetPlayerController` 0))
  (if (not (`/Game/tomWork/TemplateContent/FirstPerson/Blueprints/BP_FirstPersonCharacter.observingItem` (`self.playerRef`)))
    (if (`self.isEvidence`)
      (set `/Game/tomWork/TemplateContent/FirstPerson/Blueprints/BP_FirstPersonCharacter.observingEvidence` true (`self.playerRef`)))
    (set `/Game/tomWork/TemplateContent/FirstPerson/Blueprints/BP_FirstPersonCharacter.observableItemRef` self (`self.playerRef`))
    (`CharacterMovementComponent.DisableMovement` (`Character.CharacterMovement` (`self.playerRef`)))
    (`PlayerController.SetViewTargetWithBlend` (`GameplayStatics.GetPlayerController` 0) (`self.Camera`) (`self.zoomTime`) "VTBlend_Cubic" 1.0 false)
    (`/Game/tomWork/TemplateContent/FirstPerson/Blueprints/BP_FirstPersonCharacter.modifyMouseCursor` (`self.playerRef`) true)
    (`Controller.SetIgnoreMoveInput` _returnvalue true)
    (`Controller.SetIgnoreLookInput` _returnvalue true)
    (`KismetSystemLibrary.Delay` (+ (`self.zoomTime`) 0.5))
    (`self.raiseItem` true)))

(event `self.ReceiveBeginPlay`
  ;[0.9908 0 1] Refs
  (bind _returnvalue (`GameplayStatics.GetActorOfClass` "/Game/ollieWork/Evidence_Proto/BP_Camera.BP_Camera_C"))
  (set `self.Camera` _returnvalue)
  (set `self.startLocation` (`SceneComponent.RelativeLocation` (`self.mesh`)))
  (set `self.oriRot` (`self.K2_GetActorRotation`))
  (bind _returnvalue_2 (`GameplayStatics.GetActorOfClass` "/Game/tomWork/TemplateContent/FirstPerson/Blueprints/BP_FirstPersonCharacter.BP_FirstPersonCharacter_C"))
  (set `self.playerRef` _returnvalue_2))

(event `self.Sphere.OnComponentBeginOverlap`
  (params (OverlappedComponent :type "PrimitiveComponent Object Reference") (OtherActor :type "Actor Object Reference") (OtherComp :type "PrimitiveComponent Object Reference") (OtherBodyIndex :type Integer) (bFromSweep :type Boolean) (SweepResult :type "HitResult Structure (by ref)"))
  (bind (_returnvalue_roll _returnvalue_pitch _returnvalue_yaw) (`KismetMathLibrary.BreakRotator` (`self.K2_GetActorRotation`)))
  (bind _camera (`self.Camera`))
  (bind (_min _max) (`StaticMeshComponent.GetLocalBounds` (`self.mesh`)))
  ;[1 1 1] Set Cam Pos + Rot
  (`self.K2_SetActorLocation` _camera (`self.K2_GetActorLocation`) false false)
  (`self.K2_SetActorRotation` _camera (`KismetMathLibrary.MakeRotator` 0.0 0.0 _returnvalue_yaw) false)
  (set `self.Camera Distance` (* (.y (- _max _min)) 2.75))
  (set `SpringArmComponent.TargetArmLength` (`self.Camera Distance`) (`/Game/ollieWork/Evidence_Proto/BP_Camera.SpringArm` _camera))
  ;[0 0.1134 1] Get Item Height to dynamically set raiseItem height
  (set `self.itemHeight` (.z (- _max _min))))

(event `self.Sphere.OnComponentEndOverlap`
  (params (OverlappedComponent :type "PrimitiveComponent Object Reference") (OtherActor :type "Actor Object Reference") (OtherComp :type "PrimitiveComponent Object Reference") (OtherBodyIndex :type Integer))
  ;[1 1 1] Highlight
  (bind (_direction _newtrack_0) (`Timeline|Timeline` :!via `Reverse`)
    (:`Update`
      (`MaterialInstanceDynamic.SetScalarParameterValue` (`self.mRef`) "Thickness" (`KismetMathLibrary.Lerp` 0.0 1.0 _newtrack_0)))))

(event `raiseItem`
  (params (`Up or Down` :type Boolean))
  (bind (_startlocation_x _startlocation_y) (`KismetMathLibrary.BreakVector` (`self.startLocation`)))
  (bind _startlocation (`self.startLocation`))
  (bind _startlocation_2 (`self.startLocation`))
  (bind (_startlocation_x_2 _startlocation_y_2) (`KismetMathLibrary.BreakVector` (`self.startLocation`)))
  ;[1 1 1] Move Item Event
  (if `Up or Down`
    (set `self.endLocation` (`KismetMathLibrary.MakeVector` _startlocation_x_2 _startlocation_y_2 (* (`self.itemHeight`) 3.0)))
    (bind (_direction _newtrack_0) (`Timeline|RaiseItemTL` :!via `PlayFromStart`)
      (:`Update`
        (`SceneComponent.K2_SetRelativeLocation` (`self.mesh`) (`KismetMathLibrary.VLerp` _startlocation (+ _startlocation (`self.endLocation`)) _newtrack_0) false false))
      (:`Finished`
        (set `self.moveable` true)
        ;;[1 0 0] Set here to not let player rotate while still raising
        (set `/Game/tomWork/TemplateContent/FirstPerson/Blueprints/BP_FirstPersonCharacter.observingItem` true (`self.playerRef`))))
    (else
      (set `self.endLocation` (`KismetMathLibrary.MakeVector` _startlocation_x _startlocation_y (* (`self.itemHeight`) -3.0)))
      (set `self.currRot` (`self.K2_GetActorRotation`))
      (bind (_direction_2 _newtrack_0_2) (`Timeline|Timeline_0` :!via `PlayFromStart`)
        (:`Update`
          (`SceneComponent.K2_SetRelativeLocation` (`self.mesh`) (`KismetMathLibrary.VLerp` _startlocation_2 (+ _startlocation_2 (`self.endLocation`)) _newtrack_0_2) false false)
          (`self.K2_SetActorRotation` (`KismetMathLibrary.RLerp` (`self.currRot`) (`self.oriRot`) _newtrack_0_2 true)))
        (:`Finished`
          (set `self.moveable` false)
          (set `/Game/tomWork/TemplateContent/FirstPerson/Blueprints/BP_FirstPersonCharacter.observingItem` false (`self.playerRef`)))))))

(fn `UserConstructionScript`
  (`StaticMeshComponent.SetStaticMesh` (`self.mesh`) (`self.renderedMesh`))
  (bind _returnvalue (`PrimitiveComponent.CreateDynamicMaterialInstance` (`self.mesh`) 5 "/Game/tomWork/Materials/M_WhiteOutline.M_WhiteOutline" "None"))
  (bind _output_get (set `self.mRef` _returnvalue))
  (`MeshComponent.SetOverlayMaterial` (`self.mesh`) _output_get))