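; BP_EvidenceActor is a prototype evidence item that switches the player into a close-up observation view on interaction.
; If the player is not already observing an item, ProcInteract registers itself on the player, disables movement and look input, and modifies the mouse cursor.
; The view blends cubically to the item's Camera over ZoomTime, then RaiseItem runs after a delay slightly longer than the blend.
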(event `/Game/tomWork/Interfaces/IF_Interactable.ProcInteract`
  (params (hitComponent :type "PrimitiveComponent Object Reference"))
  (bind _returnvalue (`GameplayStatics.GetPlayerController` 0))
  (if (not (`/Game/tomWork/TemplateContent/FirstPerson/Blueprints/BP_FirstPersonCharacter.observingItem` (`self.playerRef`)))
    (set `/Game/tomWork/TemplateContent/FirstPerson/Blueprints/BP_FirstPersonCharacter.evidenceItemRef` self (`self.playerRef`))
    (`CharacterMovementComponent.DisableMovement` (`Character.CharacterMovement` (`self.playerRef`)))
    (`PlayerController.SetViewTargetWithBlend` (`GameplayStatics.GetPlayerController` 0) (`self.Camera`) (`self.zoomTime`) "VTBlend_Cubic" 1.0 false)
    (`/Game/tomWork/TemplateContent/FirstPerson/Blueprints/BP_FirstPersonCharacter.modifyMouseCursor` (`self.playerRef`) true)
    (`Controller.SetIgnoreMoveInput` _returnvalue true)
    (`Controller.SetIgnoreLookInput` _returnvalue true)
    (`KismetSystemLibrary.Delay` (+ (`self.zoomTime`) 0.5))
    (`self.raiseItem` true)))

(fn `UserConstructionScript`
  (`parent.UserConstructionScript`))