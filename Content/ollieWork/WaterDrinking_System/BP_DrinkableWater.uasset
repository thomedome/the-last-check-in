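; Drinkable water actor whose water component moves and rescales over a timeline when interacted with.
; BeginPlay caches the component's starting transform, and WaterTimeline lerps it to an offset location and end scale, setting relative location but world scale.
; The BPI interact event plays the timeline only while the Box overlap flag is set; any overlapping actor toggles that flag.
; A DrinkWater custom event also plays it but is marked unused.
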(event `self.ReceiveBeginPlay`
  (bind _full_position (`self.Full Position`))
  ;[1 0.8201 0] Sets Starting Position And Scale Of Water Component
  (set `self.Start Location` (`SceneComponent.RelativeLocation` _full_position))
  (set `self.Start Scale` (`SceneComponent.RelativeScale3D` _full_position)))

(event `Drink Water`
  ;[1 0.009362 0] Interaction Blueprint, Custom Event (Not In Use) And Timeline
  (bind (_direction _alpha) (`Timeline|Water Timeline` :!label _label)
    (:`Update`
      (bind (_returnvalue_location _returnvalue_rotation _returnvalue_scale) (`KismetMathLibrary.BreakTransform` (`KismetMathLibrary.TLerp` (`KismetMathLibrary.MakeTransform` (`self.Start Location`) (struct) (`self.Start Scale`)) (`KismetMathLibrary.MakeTransform` (+ (`self.Start Location`) (`self.End Location`)) (struct) (`self.End Scale`)) _alpha)))
      ;[0.1793 0.6722 1] Moves Water Location
      (`SceneComponent.K2_SetRelativeLocation` (`self.Full Position`) _returnvalue_location false false)
      (`SceneComponent.SetWorldScale3D` (`self.Full Position`) _returnvalue_scale))))

(event `/Game/ollieWork/Elevator_System/BPI_InteractionObjects.BPI_InteractObject`
  (params (InteractState :type String))
  ;[1 0.009362 0] Interaction Blueprint, Custom Event (Not In Use) And Timeline
  (if (`self.Is Player In Range`)
    (set `self.Interact State` InteractState)
    (goto _label)))

(event `self.Box.OnComponentBeginOverlap`
  (params (OverlappedComponent :type "PrimitiveComponent Object Reference") (OtherActor :type "Actor Object Reference") (OtherComp :type "PrimitiveComponent Object Reference") (OtherBodyIndex :type Integer) (bFromSweep :type Boolean) (SweepResult :type "HitResult Structure (by ref)"))
  ;[1 1 1] Is The Player In Range Boolean?
  (set `self.Is Player In Range` true))

(event `self.Box.OnComponentEndOverlap`
  (params (OverlappedComponent :type "PrimitiveComponent Object Reference") (OtherActor :type "Actor Object Reference") (OtherComp :type "PrimitiveComponent Object Reference") (OtherBodyIndex :type Integer))
  ;[1 1 1] Is The Player In Range Boolean?
  (set `self.Is Player In Range` false))

(fn `UserConstructionScript`)