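; Evidence paper prop that flags the first-person controller and shows an interact prompt while its collision volume is overlapped.
; BeginPlay caches the level's BP_Camera and the player controller, and creates the WBP_Interact widget.
; On overlap it also pre-positions the shared camera at the paper, copying its yaw and setting spring arm length from CameraDistance.
; Ending overlap clears the flag and removes the prompt.
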(event `self.ReceiveBeginPlay`
  (bind _returnvalue (`GameplayStatics.GetActorOfClass` "/Game/Evidence_Proto/BP_Camera.BP_Camera_C"))
  (set `self.Camera` _returnvalue)
  (bind _returnvalue_2 (`GameplayStatics.GetActorOfClass` "/Game/FirstPerson/Blueprints/BP_FirstPersonCharacter.BP_FirstPersonCharacter_C"))
  (bind _asbp_first_person_player_controller (cast `/Game/FirstPerson/Blueprints/BP_FirstPersonPlayerController` (`Pawn.GetController` _returnvalue_2)))
  (set `self.Player Controller` _asbp_first_person_player_controller)
  (bind _returnvalue_3 (`|CreateWidget` "/Game/Evidence_Proto/WBP_Interact.WBP_Interact_C"))
  (set `self.Help UI` _returnvalue_3))

(event `self.Collision.OnComponentBeginOverlap`
  (params (OverlappedComponent :type "PrimitiveComponent Object Reference") (OtherActor :type "Actor Object Reference") (OtherComp :type "PrimitiveComponent Object Reference") (OtherBodyIndex :type Integer) (bFromSweep :type Boolean) (SweepResult :type "HitResult Structure (by ref)"))
  (bind (_returnvalue_roll _returnvalue_pitch _returnvalue_yaw) (`KismetMathLibrary.BreakRotator` (`self.K2_GetActorRotation`)))
  (bind _camera (`self.Camera`))
  (set `/Game/FirstPerson/Blueprints/BP_FirstPersonPlayerController.Evidence Collision` true (`self.Player Controller`))
  (`UserWidget.AddToViewport` (`self.Help UI`) 0)
  (`self.K2_SetActorLocation` _camera (`self.K2_GetActorLocation`) false false)
  (`self.K2_SetActorRotation` _camera (`KismetMathLibrary.MakeRotator` 0.0 0.0 _returnvalue_yaw) false)
  (set `SpringArmComponent.TargetArmLength` (`self.Camera Distance`) (`/Game/Evidence_Proto/BP_Camera.SpringArm` _camera)))

(event `self.Collision.OnComponentEndOverlap`
  (params (OverlappedComponent :type "PrimitiveComponent Object Reference") (OtherActor :type "Actor Object Reference") (OtherComp :type "PrimitiveComponent Object Reference") (OtherBodyIndex :type Integer))
  (bind _help_ui (`self.Help UI`))
  (set `/Game/FirstPerson/Blueprints/BP_FirstPersonPlayerController.Evidence Collision` false (`self.Player Controller`))
  (`/Engine/EditorBlueprintResources/StandardMacros.IsValid` _help_ui
    (:`Is Valid`
      (`Widget.RemoveFromParent` _help_ui))))

(fn `UserConstructionScript`)