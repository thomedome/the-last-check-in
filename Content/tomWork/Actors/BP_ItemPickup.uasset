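; BP_ItemPickup is a world item actor that displays an item mesh and reveals a widget when the player is near.
; The construction script sets the static mesh from the Mesh field of its ItemStruct, so each instance takes its look from its item data.
; Sphere overlap events show and hide the widget, responding only to BP_FirstPersonCharacterEben.
; The graphs contain no logic for collecting the item.
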(event `self.Sphere.OnComponentBeginOverlap`
  (params (OverlappedComponent :type "PrimitiveComponent Object Reference") (OtherActor :type "Actor Object Reference") (OtherComp :type "PrimitiveComponent Object Reference") (OtherBodyIndex :type Integer) (bFromSweep :type Boolean) (SweepResult :type "HitResult Structure (by ref)"))
  (cast `/Game/Eben_Work/BP_FirstPersonCharacterEben` OtherActor)
  (`SceneComponent.SetVisibility` (`self.Widget`) true true))

(event `self.Sphere.OnComponentEndOverlap`
  (params (OverlappedComponent :type "PrimitiveComponent Object Reference") (OtherActor :type "Actor Object Reference") (OtherComp :type "PrimitiveComponent Object Reference") (OtherBodyIndex :type Integer))
  (cast `/Game/Eben_Work/BP_FirstPersonCharacterEben` OtherActor)
  (`SceneComponent.SetVisibility` (`self.Widget`) false true))

(fn `UserConstructionScript`
  (`StaticMeshComponent.SetStaticMesh` (`self.StaticMesh`) (`.Mesh_8_AF4F76EA42B34DB8F2EC43A61CF27893` (break `/Game/tomWork/DataTypes/Struct_Item` (`self.itemStruct`)))))