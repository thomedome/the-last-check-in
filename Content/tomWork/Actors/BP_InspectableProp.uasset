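; BP_InspectableProp is a prop that fades in a white outline when something enters its sphere trigger, marking it as inspectable.
; The construction script assigns the configurable mesh and sets a dynamic M_WhiteOutline instance as its overlay material.
; Sphere begin overlap plays a timeline that drives the material's Thickness parameter, and end overlap reverses it.
; Overlaps are not filtered by actor type.
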(event `self.Sphere.OnComponentBeginOverlap`
  (params (OverlappedComponent :type "PrimitiveComponent Object Reference") (OtherActor :type "Actor Object Reference") (OtherComp :type "PrimitiveComponent Object Reference") (OtherBodyIndex :type Integer) (bFromSweep :type Boolean) (SweepResult :type "HitResult Structure (by ref)"))
  (bind (_direction _newtrack_0) (`Timeline|Timeline` :!label _label)
    (:`Update`
      (`MaterialInstanceDynamic.SetScalarParameterValue` (`self.mRef`) "Thickness" (`KismetMathLibrary.Lerp` 0.0 1.0 _newtrack_0)))))

(event `self.Sphere.OnComponentEndOverlap`
  (params (OverlappedComponent :type "PrimitiveComponent Object Reference") (OtherActor :type "Actor Object Reference") (OtherComp :type "PrimitiveComponent Object Reference") (OtherBodyIndex :type Integer))
  (goto _label :!via `Reverse`))

(fn `UserConstructionScript`
  (`StaticMeshComponent.SetStaticMesh` (`self.StaticMesh`) (`self.meshDisplayed`))
  (bind _returnvalue (`PrimitiveComponent.CreateDynamicMaterialInstance` (`self.StaticMesh`) 5 "/Game/tomWork/Materials/M_WhiteOutline.M_WhiteOutline" "None"))
  (`MeshComponent.SetOverlayMaterial` (`self.StaticMesh`) _returnvalue)
  (set `self.mRef` _returnvalue))