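; BP_JournalTest is a test journal actor that shows an interaction prompt and opens a journal screen on proximity.
; BeginPlay copies InteractionText into the WBP_InteractionPrompt on its Widget component.
; Box overlap unhides the prompt and immediately adds a new WBP_journal to the viewport for player 0, with no input or actor check.
; End overlap hides the prompt and removes the journal.
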(event `self.ReceiveBeginPlay`
  ;[0.2984 0 0.1419] Set Above Text
  (bind _aswbp_interaction_prompt (cast `/Game/Eben_Work/WBP_InteractionPrompt` (`WidgetComponent.GetWidget` (`self.Widget`))))
  (set `/Game/Eben_Work/WBP_InteractionPrompt.Text` (`self.InteractionText`) _aswbp_interaction_prompt))

(event `self.Box.OnComponentBeginOverlap`
  (params (OverlappedComponent :type "PrimitiveComponent Object Reference") (OtherActor :type "Actor Object Reference") (OtherComp :type "PrimitiveComponent Object Reference") (OtherBodyIndex :type Integer) (bFromSweep :type Boolean) (SweepResult :type "HitResult Structure (by ref)"))
  ;[0 0.1704 0.1567] Show and Hide text
  (`SceneComponent.SetHiddenInGame` (`self.Widget`) false false)
  (bind _returnvalue (`|CreateWidget` "/Game/Eben_Work/journal/WBP_journal.WBP_journal_C" (`GameplayStatics.GetPlayerController` 0)))
  (`UserWidget.AddToViewport` _returnvalue 0))

(event `self.Box.OnComponentEndOverlap`
  (params (OverlappedComponent :type "PrimitiveComponent Object Reference") (OtherActor :type "Actor Object Reference") (OtherComp :type "PrimitiveComponent Object Reference") (OtherBodyIndex :type Integer))
  ;[0 0.1704 0.1567] Show and Hide text
  (`SceneComponent.SetHiddenInGame` (`self.Widget`) true false)
  (`Widget.RemoveFromParent` (stale `self.Box.OnComponentBeginOverlap` _returnvalue)))

(fn `UserConstructionScript`)