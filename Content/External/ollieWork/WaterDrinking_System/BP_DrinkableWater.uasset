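; BP_DrinkableWater is a water actor whose water component moves and rescales when drunk through interaction.
; BeginPlay caches the FullPosition component's starting relative location and scale.
; ProcInteract plays WaterTimeline, as does DrinkWater, which is noted as unused.
; The timeline alpha lerps location by the EndLocation offset and scale toward EndScale, applying scale in world space despite caching it as relative.
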(event `self.ReceiveBeginPlay`
  (bind _full_position (`self.Full Position`))
  ;[1 0.8201 0] Sets Starting Position And Scale Of Water Component
  (set `self.Start Location` (`SceneComponent.RelativeLocation` _full_position))
  (set `self.Start Scale` (`SceneComponent.RelativeScale3D` _full_position)))

(event `Drink Water`
  ;[1 0.009362 0] Interaction Blueprint, Custom Event (Not In Use) And Timeline
  (bind (_direction _alpha) (`Timeline|Water Timeline` :!label _label)
    (:`Update`
      (bind (_returnvalue_location _returnvalue_rotation _returnvalue_scale) (`KismetMathLibrary.BreakTransform` (`KismetMathLibrary.TLerp` (`KismetMathLibrary.MakeTransform` (`self.Start Location`) (struct) (`self.Start Scale`)) (`KismetMathLibrary.MakeTransform` (+ (`self.Start Location`) (`self.End Location`)) (struct) (`self.End Scale`)) _alpha)))
      ;[0.1793 0.6722 1] Moves Water Location
      (`SceneComponent.K2_SetRelativeLocation` (`self.Full Position`) _returnvalue_location false false)
      (`SceneComponent.SetWorldScale3D` (`self.Full Position`) _returnvalue_scale))))

(event `/Game/tomWork/Interfaces/IF_Interactable.ProcInteract`
  (params (hitComponent :type "PrimitiveComponent Object Reference"))
  ;[1 0.009362 0] Interaction Blueprint, Custom Event (Not In Use) And Timeline
  (goto _label))

(fn `UserConstructionScript`)