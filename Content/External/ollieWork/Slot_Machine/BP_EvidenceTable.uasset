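; BP_EvidenceTable is an interactable table that spawns a reward once the player has collected the newspaper.
; BeginPlay caches the BP_FirstPersonCharacterOllie player and an existing BP_Reward, and disables physics on that reward's cylinder.
; The interface interact event checks the player's NewsPaperCollected flag, spawns a new BP_Reward at the table's Plane location when true, and prints a debug result.
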(event `self.ReceiveBeginPlay`
  (bind _returnvalue (`GameplayStatics.GetActorOfClass` "/Game/ollieWork/FirstPerson/Blueprints/BP_FirstPersonCharacterOllie.BP_FirstPersonCharacterOllie_C"))
  (bind _output_get (set `self.Player Ref` _returnvalue))
  (bind _returnvalue_2 (`GameplayStatics.GetActorOfClass` "/Game/ollieWork/Slot_Machine/BP_Reward.BP_Reward_C"))
  (bind _output_get_2 (set `self.Reward Ref` _returnvalue_2))
  (`PrimitiveComponent.SetSimulatePhysics` (`/Game/ollieWork/Slot_Machine/BP_Reward.Cylinder` _output_get_2) false))

(event `/Game/ollieWork/Elevator_System/BPI_InteractionObjects.BPI_InteractObject`
  (params (InteractState :type String))
  (set `self.Interact State` InteractState)
  (if (`/Game/ollieWork/FirstPerson/Blueprints/BP_FirstPersonCharacterOllie.NewsPaperCollected?` (stale `self.ReceiveBeginPlay` _output_get))
    (`|SpawnActorFromClass` "/Game/ollieWork/Slot_Machine/BP_Reward.BP_Reward_C" (`KismetMathLibrary.MakeTransform` (`SceneComponent.K2_GetComponentLocation` (`self.Plane`))) "Undefined" "MultiplyWithRoot" null null)
    (`KismetSystemLibrary.PrintString` "True")
    (else
      (`KismetSystemLibrary.PrintString` "False"))))

(fn `UserConstructionScript`)