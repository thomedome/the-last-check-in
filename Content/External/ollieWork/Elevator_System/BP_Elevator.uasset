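; Elevator actor that moves between numbered floors and animates its two sliding doors.
; On BeginPlay it maps every BP_ElevatorFloorIndicator in the level by floor number, so all elevators would share one set of stops.
; A goToFloor call takes the indicator's location, closes the doors, then lerps the actor there on a timeline.
; Delays sequence the reversed door timeline on arrival and release a cooldown that blocks overlapping trips.
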(event `goToFloor`
  (params (DestinationFloor :type Integer))
  ;[1 1 1] Go To Floor Event
  (if (not (== DestinationFloor (`self.currentFloor`)))
    (bind _output_get (set `self.Destination Floor` DestinationFloor))
    (bind (_value _returnvalue) (`BlueprintMapLibrary.Map_Find` (`self.FloorToIndicatorMap`) _output_get))
    (if _returnvalue
      (set `self.Target Floor` (`self.K2_GetActorLocation` _value))
      (`self.TransferFloors`)
      (set `self.currentFloor` (`self.Destination Floor`)))))

(event `self.ReceiveBeginPlay`
  ;[1 0.8557 0] Sets Initial Vector Values / Locations
  (set `self.Current Location` (`SceneComponent.K2_GetComponentLocation` (`self.Cube`)))
  (set `self.Left Door Open Location` (`SceneComponent.RelativeLocation` (`self.Left Door`)))
  (set `self.Right Door Open Location` (`SceneComponent.RelativeLocation` (`self.Right Door`)))
  ;[0.005836 0 1] Populate F->I Map - These store locations of each floor. Must remain in line to elevator on Z axis (Up/Down) -- If there is going to be more than one elevator in the game, then this will break horribly.
  ; Talk to Tom before changing this!
  (bind _outactors (`GameplayStatics.GetAllActorsOfClass` "/Game/ollieWork/Elevator_System/BP_ElevatorFloorIndicator.BP_ElevatorFloorIndicator_C"))
  (for _array_element _outactors
    (`BlueprintMapLibrary.Map_Add` (`self.FloorToIndicatorMap`) (`/Game/ollieWork/Elevator_System/BP_ElevatorFloorIndicator.Floor` _array_element) _array_element)))

(event `TransferFloors`
  ;[1 0.04688 0.04688] Lift Movement Timeline/Event
  (if (not (`self.Lift Cooldown`))
    (`self.Close Doors`)
    (set `self.Lift Cooldown` true)
    (`KismetSystemLibrary.Delay` 2.5)
    (bind (_direction _alpha) (`Timeline|Floor Timeline` :!via `PlayFromStart`)
      (:`Update`
        (`self.K2_SetActorLocation` (`KismetMathLibrary.VLerp` (`self.Current Location`) (`self.Target Floor`) _alpha)))
      (:`Finished`
        (`KismetSystemLibrary.Delay` 0.7)
        (`self.Open Doors`)
        (`KismetSystemLibrary.Delay` 3.0)
        (set `self.Lift Cooldown` false)
        (set `self.Current Location` (`SceneComponent.K2_GetComponentLocation` (`self.Cube`)))))))

(event `Close Doors`
  ;[0.02322 0.8803 1] Doors Opening And Closing
  (if (not (`self.Lift Cooldown`))
    (bind (_direction _door_alpha) (`Timeline|Door Timeline` :!label _label)
      (:`Update`
        (`|ExecutionSequence`
          (:`then_0`
            (`SceneComponent.K2_SetRelativeLocation` (`self.Left Door`) (`KismetMathLibrary.VLerp` (`self.Left Door Open Location`) (`self.Left Door Closed Location`) _door_alpha) false false))
          (:`then_1`
            (`SceneComponent.K2_SetRelativeLocation` (`self.Right Door`) (`KismetMathLibrary.VLerp` (`self.Right Door Open Location`) (`self.Right Floor Closed Location`) _door_alpha) false false)))))))

(event `Open Doors`
  ;[0.02322 0.8803 1] Doors Opening And Closing
  (goto _label :!via `Reverse`))

(fn `UserConstructionScript`)