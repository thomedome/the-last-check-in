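; BP_Door is an interactable hinged door actor that swings open when used, unless it is locked or already open.
; ProcInteract checks the open and locked flags, then calls Open, which plays a timeline that lerps the door mesh yaw to an open angle and marks it open when finished.
; On BeginPlay it writes its door number into a WBP_DoorNumber widget component.
; The file has no closing logic.
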(event `/Game/tomWork/Interfaces/IF_Interactable.ProcInteract`
  (if (`self.isOpen`)
    _
    (elif (not (`self.doorLocked`))
      (`self.Open`))))

(event `self.ReceiveBeginPlay`
  (bind _aswbp_door_number (cast `/Game/tomWork/Widgets/WBP_DoorNumber` (`WidgetComponent.GetWidget` (`self.Widget`))))
  (`/Game/tomWork/Widgets/WBP_DoorNumber.setText` _aswbp_door_number (`self.doorNumber`)))

(event `Open`
  (bind (_direction _newtrack_0) (`Timeline|rotateDoor`)
    (:`Update`
      (`SceneComponent.K2_SetRelativeRotation` (`self.door`) (`KismetMathLibrary.MakeRotator` 0.0 0.0 (`KismetMathLibrary.Lerp` 0.0 -85.0 _newtrack_0)) false false))
    (:`Finished`
      (set `self.isOpen` true))))

(fn `UserConstructionScript`)