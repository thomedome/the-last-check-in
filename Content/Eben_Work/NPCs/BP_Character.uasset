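; NPC Blueprint that opens a two-stage dialogue based on the newspaper-scrap evidence the player has collected.
; Box overlap toggles a prompt widget; BeginPlay sets its text, the NPC's skin and the player reference.
; On interact, the highest scrap number sets the dialogue stage, appended to the NPC name as dialogue key, then the game pauses.
; Without scraps, only Jake opens dialogue, using his plain name.
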(event `/Game/tomWork/Interfaces/IF_Interactable.ProcInteract`
  (params (hitComponent :type "PrimitiveComponent Object Reference"))
  (bind _dialoguenum (`self.DialogueNum`))
  (bind _name (`self.Name`))
  ;[1 0.4108 0] Interaction
  (bind _highestpaperint (`self.decideHighestEvidence` (`/Game/tomWork/TemplateContent/FirstPerson/Blueprints/BP_FirstPersonCharacter.evidenceArr` (`self.PlayerRef`))))
  (bind _result (`/Engine/EditorBlueprintResources/StandardMacros.IncrementInt` _highestpaperint)
    (:`  `
      (set `self.DialogueNum` _result)
      (bind _returnvalue (`|CreateWidget` "/Game/Eben_Work/Dialogue/WBP_TwoStageDialogue.WBP_TwoStageDialogue_C" (`GameplayStatics.GetPlayerController` 0)))
      (set `/Game/Eben_Work/Dialogue/WBP_TwoStageDialogue.ReputationDialogue` _name _returnvalue)
      (if (< _dialoguenum 2)
        (if (== (`self.Name`) "Jake")
          (`UserWidget.AddToViewport` _returnvalue 0 :!label _label)
          (`/Game/tomWork/TemplateContent/FirstPerson/Blueprints/BP_FirstPersonCharacter.modifyMouseCursor` (`self.PlayerRef`) true)
          (`GameplayStatics.SetGamePaused` true))
        (else
          (set `/Game/Eben_Work/Dialogue/WBP_TwoStageDialogue.ReputationDialogue` (`KismetStringLibrary.Conv_StringToName` (`KismetStringLibrary.Concat_StrStr` (`KismetStringLibrary.Conv_NameToString` _name) (`KismetStringLibrary.Conv_IntToString` _dialoguenum))) _returnvalue)
          (goto _label))))))

(event `self.ReceiveBeginPlay`
  ;[0.2984 0 0.1419] Set Above Text
  (bind _aswbp_interaction_prompt (cast `/Game/Eben_Work/WBP_InteractionPrompt` (`WidgetComponent.GetWidget` (`self.Widget`))))
  (set `/Game/Eben_Work/WBP_InteractionPrompt.Text` (`self.InteractionText`) _aswbp_interaction_prompt)
  (bind _returnvalue (`GameplayStatics.GetActorOfClass` "/Game/tomWork/TemplateContent/FirstPerson/Blueprints/BP_FirstPersonCharacter.BP_FirstPersonCharacter_C"))
  (set `self.PlayerRef` _returnvalue)
  (`SkeletalMeshComponent.SetSkeletalMeshAsset` (`self.male03_1`) (`self.Skin`)))

(event `self.Box.OnComponentBeginOverlap`
  (params (OverlappedComponent :type "PrimitiveComponent Object Reference") (OtherActor :type "Actor Object Reference") (OtherComp :type "PrimitiveComponent Object Reference") (OtherBodyIndex :type Integer) (bFromSweep :type Boolean) (SweepResult :type "HitResult Structure (by ref)"))
  ;[0 0.1704 0.1567] Show and Hide text
  (`SceneComponent.SetHiddenInGame` (`self.Widget`) false false))

(event `self.Box.OnComponentEndOverlap`
  (params (OverlappedComponent :type "PrimitiveComponent Object Reference") (OtherActor :type "Actor Object Reference") (OtherComp :type "PrimitiveComponent Object Reference") (OtherBodyIndex :type Integer))
  ;[0 0.1704 0.1567] Show and Hide text
  (`SceneComponent.SetHiddenInGame` (`self.Widget`) true false))

(fn `decideHighestEvidence`
  (params (array :type "Array of /Game/tomWork/DataTypes/Struct_Evidence Structure"))
  (returns (highestpaperInt :type Integer))
  (locals (highestNewspaper :type Integer) (tempNewspaper :type Integer))
  (for _array_element array
    (switch `/Game/tomWork/DataTypes/Enum_EvidenceID` (`.ID_9_F0104CB042C99B5DD9164B8E041E69F9` (break `/Game/tomWork/DataTypes/Struct_Evidence` _array_element))
      (:`NewEnumerator0`
        (set `local.tempNewspaper` 1))
      (:`NewEnumerator1`
        (set `local.tempNewspaper` 2))
      (:`NewEnumerator2`
        (set `local.tempNewspaper` 3))
      (:`NewEnumerator3`
        (set `local.tempNewspaper` 4)))
    (if (< (`local.highestNewspaper`) (`local.tempNewspaper`))
      (set `local.highestNewspaper` (`local.tempNewspaper`))))
  (return (`local.highestNewspaper`)))

(fn `UserConstructionScript`)